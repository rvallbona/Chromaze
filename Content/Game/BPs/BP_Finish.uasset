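; BP_Finish is a red or blue goal trigger for the player, tinted at BeginPlay through dynamic materials according to InitBlue.
; A color-matched player overlapping it while a same-Level BP_Door is closed sets PlayerCollision, plays a sound, calls ActivateDog on BP_GameManager, and lights the neon and player's eye.
; When that player leaves, the flag, neon and eye switch off.
; EncenderCables and ApagarCables recolor or blacken color-matched cables, but are not called here.
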(event OnComponentBeginOverlap(trigger)
  (params (OverlappedComponent :type Primitive%20Component%20Object%20Reference) (OtherActor :type Actor%20Object%20Reference) (OtherComp :type Primitive%20Component%20Object%20Reference) (OtherBodyIndex :type Integer) (bFromSweep :type Boolean) (SweepResult :type Hit%20Result%20Structure%20%28by%20ref%29))
  ;[1 1 1] Check Collision
  (bind _asbp_player (Utilities|Casting|CastToBP_Player OtherActor))
  (if (== (Variables|/Game/Game/Players/Blueprints/BP_Player.BP_Player_C|GetisBlue _asbp_player) (Variables|Default|GetcurrentColorIsblue))
    (bind _outactors (Actor|GetAllActorsOfClass "/Game/Game/BPs/BP_Door.BP_Door_C"))
    (for _array_element _outactors
      (bind _asbp_door (Utilities|Casting|CastToBP_Door _array_element))
      (if (== (Variables|/Game/Game/BPs/BP_Door.BP_Door_C|Getlevel _asbp_door) (Variables|Default|Getlevel))
        (if (not (Variables|/Game/Game/BPs/BP_Door.BP_Door_C|Getopen _asbp_door))
          (Audio|PlaySoundatLocation "/Game/Game/Sounds/FX/Button_Cue.Button_Cue" (Transformation|GetActorLocation) "0, 0, 0" 1.0 1.0 0.0 0 0 0 0)
          (Variables|Default|SetplayerCollision true)
          (bind _returnvalue (Actor|GetActorOfClass "/Game/Game/Levels/BP_GameManager.BP_GameManager_C"))
          (Default|ActivateDog _returnvalue)
          (bind _returnvalue_2 (Rendering|Material|CreateDynamicMaterialInstance (Variables|Default|GetMEtaModel) 2 "/Game/Game/Materials/MI_dynamic_blueRed_neon.MI_dynamic_blueRed_neon" "None" :!class /Script/Engine.PrimitiveComponent))
          (bind _output_get (Variables|Default|SetdynamicColor _returnvalue_2))
          (if (Variables|Default|GetcurrentColorIsblue)
            (Rendering|Material|SetVectorParameterValue _output_get "BaseColor" "(R=0.000000,G=0.000000,B=1.000000,A=1.000000)" :!class /Script/Engine.MaterialInstanceDynamic)
            (else
              (Rendering|Material|SetVectorParameterValue _output_get "BaseColor" "(R=1.000000,G=0.000000,B=0.000000,A=1.000000)" :!class /Script/Engine.MaterialInstanceDynamic)))
          (Default|EncenderOjo _asbp_player))))))

(event OnComponentEndOverlap(trigger)
  (params (OverlappedComponent :type Primitive%20Component%20Object%20Reference) (OtherActor :type Actor%20Object%20Reference) (OtherComp :type Primitive%20Component%20Object%20Reference) (OtherBodyIndex :type Integer))
  ;[1 1 1] Out Collision
  (bind _asbp_player (Utilities|Casting|CastToBP_Player OtherActor))
  (if (== (Variables|/Game/Game/Players/Blueprints/BP_Player.BP_Player_C|GetisBlue _asbp_player) (Variables|Default|GetcurrentColorIsblue))
    (Variables|Default|SetplayerCollision false)
    (bind _returnvalue (Rendering|Material|CreateDynamicMaterialInstance (Variables|Default|GetMEtaModel) 2 "/Game/Game/Materials/MI_dynamic_blueRed_neon.MI_dynamic_blueRed_neon" "None" :!class /Script/Engine.PrimitiveComponent))
    (Rendering|Material|SetVectorParameterValue _returnvalue "BaseColor" "(R=0.000000,G=0.000000,B=0.000000,A=1.000000)" :!class /Script/Engine.MaterialInstanceDynamic)
    (Default|ApagarOjo _asbp_player)))

(event EventBeginPlay
  ;[1 1 1] Init box color
  (bind _returnvalue (Rendering|Material|CreateDynamicMaterialInstance (Variables|Default|GetMEtaModel) 0 "/Game/Game/Materials/MI_dynamic_blueRed.MI_dynamic_blueRed" "None" :!class /Script/Engine.PrimitiveComponent))
  (bind _output_get (Variables|Default|SetdynamicColor _returnvalue))
  (if (Variables|Default|Getinit_blue)
    (Rendering|Material|SetVectorParameterValue _output_get "BaseColor" "(R=0.000000,G=0.000000,B=1.000000,A=1.000000)" :!class /Script/Engine.MaterialInstanceDynamic)
    (Variables|Default|SetcurrentColorIsBlue true)
    (bind _returnvalue_2 (Rendering|Material|CreateDynamicMaterialInstance (Variables|Default|GetMEtaModel) 1 "/Game/Game/Materials/M_Glass_Dynamic.M_Glass_Dynamic" "None" :!class /Script/Engine.PrimitiveComponent))
    (Rendering|Material|SetVectorParameterValue _returnvalue_2 "ColorGlass" "(R=0.000000,G=0.000000,B=1.000000,A=1.000000)" :!class /Script/Engine.MaterialInstanceDynamic)
    (else
      (Rendering|Material|SetVectorParameterValue _output_get "BaseColor" "(R=1.000000,G=0.000000,B=0.000000,A=1.000000)" :!class /Script/Engine.MaterialInstanceDynamic)
      (Variables|Default|SetcurrentColorIsBlue false)
      (bind _returnvalue_3 (Rendering|Material|CreateDynamicMaterialInstance (Variables|Default|GetMEtaModel) 1 "/Game/Game/Materials/M_Glass_Dynamic.M_Glass_Dynamic" "None" :!class /Script/Engine.PrimitiveComponent))
      (Rendering|Material|SetVectorParameterValue _returnvalue_3 "ColorGlass" "(R=1.000000,G=0.000000,B=0.000000,A=1.000000)" :!class /Script/Engine.MaterialInstanceDynamic))))

(fn ConstructionScript)

(fn EncenderCables
  (bind _currentcolorisblue (Variables|Default|GetcurrentColorIsblue))
  (bind _currentcolorisblue_2 (Variables|Default|GetcurrentColorIsblue))
  (bind _outactors (Actor|GetAllActorsOfClass "/Game/Game/BPs/Cables/BP_CableRecto.BP_CableRecto_C"))
  (for _array_element _outactors
    (if (== (Variables|/Game/Game/BPs/Cables/BP_CableRecto.BP_CableRecto_C|GetIsBlue _array_element) _currentcolorisblue)
      (if _currentcolorisblue
        (Default|ChangetoBlue _array_element)
        (else
          (Default|ChangetoRed _array_element)))
      (bind _outactors_2 (Actor|GetAllActorsOfClass "/Game/Game/BPs/Cables/BP_CableCurva.BP_CableCurva_C"))
      (for _array_element_2 _outactors_2
        (if (== (Variables|/Game/Game/BPs/Cables/BP_CableCurva.BP_CableCurva_C|GetIsBlue _array_element_2) _currentcolorisblue_2)
          (if _currentcolorisblue_2
            (Default|ChangetoBlue _array_element_2)
            (else
              (Default|ChangetoRed _array_element_2))))))))

(fn ApagarCables
  (bind _outactors (Actor|GetAllActorsOfClass "/Game/Game/BPs/Cables/BP_CableRecto.BP_CableRecto_C"))
  (for _array_element _outactors
    (if (== (Variables|/Game/Game/BPs/Cables/BP_CableRecto.BP_CableRecto_C|GetIsBlue _array_element) (Variables|Default|GetcurrentColorIsblue))
      (Default|ChangetoBlack _array_element)
      (bind _outactors_2 (Actor|GetAllActorsOfClass "/Game/Game/BPs/Cables/BP_CableCurva.BP_CableCurva_C"))
      (for _array_element_2 _outactors_2
        (if (== (Variables|/Game/Game/BPs/Cables/BP_CableCurva.BP_CableCurva_C|GetIsBlue _array_element_2) (Variables|Default|GetcurrentColorIsblue))
          (Default|ChangetoBlack _array_element_2))))))