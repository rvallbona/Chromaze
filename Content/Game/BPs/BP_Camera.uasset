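; BP_Camera is a single camera actor that jumps between preset transforms, giving each level its own set of switchable views.
; SetLevelCameras sums per-level camera counts to get that level's index range, and SwapNextCamera wraps forward or backward within it.
; Each switch plays a sound, briefly flashes an alternate post-process effect and updates Widget_Camera widgets.
; FocusLastCamera jumps to the level's exit-door camera.
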(event Custom|SwapNextCamera
  (params (nextCamera :type Boolean))
  ;[1 1 1] NextCamera
  (if nextCamera
    (bind _result (Math|Integer|IncrementInt (Variables|Default|GetcameraArrayPos))
      (:%20%20
        (if (> _result (Variables|Default|GetlastCamera))
          (Variables|Default|SetcameraArrayPos (Variables|Default|GetfirstCamera)))))
    (else
      (bind _result_2 (Math|Integer|DecrementInt (Variables|Default|GetcameraArrayPos))
        (:%20%20
          (if (< _result_2 (Variables|Default|GetfirstCamera))
            (Variables|Default|SetcameraArrayPos (Variables|Default|GetlastCamera)))))))
  (bind _foundwidgets (Widget|GetAllWidgetsOfClass "/Game/Game/UI/Camera/Widget_Camera.Widget_Camera_C" true))
  (for _array_element _foundwidgets
    (Variables|/Script/Engine.CameraComponent|SetPostProcessSettings (Variables|Default|GetCamera) (Utilities|Array|Get(acopy) (Variables|Default|GetpostProcessSet) 1))
    (Audio|PlaySound2D "/Game/Game/Sounds/FX/switchCamera_Cue.switchCamera_Cue" 1.0 1.0 0.0 0 0)
    (Utilities|FlowControl|Delay 0.15)
    (Variables|/Script/Engine.CameraComponent|SetPostProcessSettings (Variables|Default|GetCamera) (Utilities|Array|Get(acopy) (Variables|Default|GetpostProcessSet)))
    (Default|SwitchCamera _array_element (Variables|Default|GetcameraArrayPos)))
  (Transformation|SetActorTransform (Utilities|Array|Get(acopy) (Variables|Default|GetcameraTransforms) (Variables|Default|GetcameraArrayPos)) true))

(event Custom|SetLevelCameras
  (params (level :type Integer))
  ;[1 1 1] Receive the level and set the cameras
  (Variables|Default|SetfirstCamera 0)
  (if (> level 0)
    (for _index (range 0 (- level 1))
      (Variables|Default|SetfirstCamera (+ (Utilities|Array|Get(acopy) (Variables|Default|GetlevelCameras) _index) (Variables|Default|GetfirstCamera)))))
  (bind _result (Math|Integer|DecrementInt (+ (Variables|Default|GetfirstCamera) (Utilities|Array|Get(acopy) (Variables|Default|GetlevelCameras) level)))
    (:%20%20
      (bind _output_get (Variables|Default|SetlastCamera _result))
      (Variables|Default|SetcameraArrayPos _output_get)
      (CallFunction|SwapNextCamera true))))

(event Custom|FocusLastCamera
  ;[1 1 1] Focus last camera (exit door Camera)
  (if (!= (Variables|Default|GetcameraArrayPos) (Variables|Default|GetlastCamera))
    (bind _output_get (Variables|Default|SetcameraArrayPos (Variables|Default|GetlastCamera)))
    (Math|Integer|DecrementInt _output_get
      (:%20%20
        (CallFunction|SwapNextCamera true)))))

(event EventBeginPlay
  ;[1 1 1] Init Camera Pos
  (Transformation|SetActorTransform (Utilities|Array|Get(acopy) (Variables|Default|GetcameraTransforms) (Variables|Default|GetcameraArrayPos)))
  (CallFunction|SetLevelCameras)
  ;[1 1 1] Init Camera effect
  (Variables|/Script/Engine.CameraComponent|SetPostProcessSettings (Variables|Default|GetCamera) (Utilities|Array|Get(acopy) (Variables|Default|GetpostProcessSet))))

(fn ConstructionScript)