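; Red/blue physics box that respawns an overlapping BP_Player whose color differs from its own.
; A dynamic material instance shows the color, set from InitBlue at start and toggled by SwapColor.
; Overlap by BP_Perro (the dog) turns off physics simulation so it cannot push the box; other overlaps reapply the configured setting.
; Respawn plays a sound, spawns a replacement at the initial transform, attempts color carry-over, and destroys itself.
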(event OnComponentBeginOverlap(Box)
  (params (OverlappedComponent :type Primitive%20Component%20Object%20Reference) (OtherActor :type Actor%20Object%20Reference) (OtherComp :type Primitive%20Component%20Object%20Reference) (OtherBodyIndex :type Integer) (bFromSweep :type Boolean) (SweepResult :type Hit%20Result%20Structure%20%28by%20ref%29))
  (bind _staticmesh (Variables|Default|GetStaticMesh))
  ;[1 1 1] Player Collision
  (bind _asbp_player (Utilities|Casting|CastToBP_Player OtherActor)
    (:then
      (Physics|SetSimulatePhysics (Variables|Default|GetStaticMesh) (Variables|Default|GetsimulatePhysics))
      (if (!= (Variables|/Game/Game/Players/Blueprints/BP_Player.BP_Player_C|GetisBlue _asbp_player) (Variables|Default|GetcurrentColorIsBlue))
        (Default|Respawn _asbp_player)))
    (:CastFailed
      ;[1 1 1] perro no empuja caja
      (Utilities|Casting|CastToBP_Perro OtherActor
        (:then
          (Physics|SetSimulatePhysics _staticmesh false))
        (:CastFailed
          (Physics|SetSimulatePhysics _staticmesh (Variables|Default|GetsimulatePhysics)))))))

(event Custom|SwapColor
  (bind _dynamiccolor (Variables|Default|GetdynamicColor))
  ;[1 1 1] Swap Color Function
  (if (Variables|Default|GetcurrentColorIsBlue)
    (Rendering|Material|SetVectorParameterValue _dynamiccolor "BaseColor" "(R=1.000000,G=0.000000,B=0.000000,A=1.000000)" :!class /Script/Engine.MaterialInstanceDynamic)
    (Variables|Default|SetcurrentColorIsBlue false)
    (else
      (Rendering|Material|SetVectorParameterValue _dynamiccolor "BaseColor" "(R=0.000000,G=0.000000,B=1.000000,A=1.000000)" :!class /Script/Engine.MaterialInstanceDynamic)
      (Variables|Default|SetcurrentColorIsBlue true))))

(event Custom|Respawn
  (bind _currentcolorisblue (Variables|Default|GetcurrentColorIsBlue))
  ;[1 1 1] Respawn
  (Audio|PlaySoundatLocation "/Game/Game/Sounds/FX/Respawn_Cue.Respawn_Cue" (.location (Variables|Default|GetinitTransform)) "0, 0, 0" 1.0 1.0 0.0 0 0 0 0)
  (bind _returnvalue (Game|SpawnActorfromClass "BP_box_nofreeze_C" (Variables|Default|GetinitTransform) "Undefined" 0 0))
  (if _currentcolorisblue
    _
    (else
      (CallFunction|SwapColor _returnvalue)))
  (Variables|BP_box_nofreeze_C|Setinit_blue _returnvalue _currentcolorisblue)
  (Physics|SetSimulatePhysics (Variables|BP_box_nofreeze_C|GetStaticMesh _returnvalue) (Variables|Default|GetsimulatePhysics))
  (Actor|DestroyActor self))

(event EventBeginPlay
  ;[1 1 1] Init box color
  (bind _returnvalue (Rendering|Material|CreateDynamicMaterialInstance (Variables|Default|GetStaticMesh) 0 "/Game/Game/Materials/MI_dynamic_blueRed.MI_dynamic_blueRed" "None" :!class /Script/Engine.PrimitiveComponent))
  (bind _output_get (Variables|Default|SetdynamicColor _returnvalue))
  (if (Variables|Default|Getinit_blue)
    (Rendering|Material|SetVectorParameterValue _output_get "BaseColor" "(R=0.000000,G=0.000000,B=1.000000,A=1.000000)" :!class /Script/Engine.MaterialInstanceDynamic)
    (Variables|Default|SetcurrentColorIsBlue true)
    (else
      (Rendering|Material|SetVectorParameterValue _output_get "BaseColor" "(R=1.000000,G=0.000000,B=0.000000,A=1.000000)" :!class /Script/Engine.MaterialInstanceDynamic)
      (Variables|Default|SetcurrentColorIsBlue false)))
  ;[1 1 1] Set gravity
  (Physics|SetSimulatePhysics (Variables|Default|GetStaticMesh) (Variables|Default|GetsimulatePhysics))
  ;[1 1 1] Save Init Transform
  (Variables|Default|SetinitTransform (Transformation|GetActorTransform)))

(fn ConstructionScript)