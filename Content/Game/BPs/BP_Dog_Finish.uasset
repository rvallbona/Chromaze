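; Finish trigger for the dog (BP_Perro) that opens the doors of its level.
; On overlap it plays a button sound, sets PlayerCollision, opens every BP_Door with a matching Level and turns the goal model's neon material green for each match.
; Leaving clears only the collision flag.
; A separate ActivateFinish event turns the model's base material green, also through a dynamic material instance.
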(event OnComponentBeginOverlap(trigger)
  (params (OverlappedComponent :type Primitive%20Component%20Object%20Reference) (OtherActor :type Actor%20Object%20Reference) (OtherComp :type Primitive%20Component%20Object%20Reference) (OtherBodyIndex :type Integer) (bFromSweep :type Boolean) (SweepResult :type Hit%20Result%20Structure%20%28by%20ref%29))
  ;[1 1 1] Check Collision
  (Utilities|Casting|CastToBP_Perro OtherActor)
  (Audio|PlaySoundatLocation "/Game/Game/Sounds/FX/Button_Cue.Button_Cue" (Transformation|GetActorLocation) "0, 0, 0" 1.0 1.0 0.0 0 0 0 0)
  (Variables|Default|SetplayerCollision true)
  (bind _outactors (Actor|GetAllActorsOfClass "/Game/Game/BPs/BP_Door.BP_Door_C"))
  (for _array_element _outactors
    (if (== (Variables|/Game/Game/BPs/BP_Door.BP_Door_C|Getlevel _array_element) (Variables|Default|Getlevel))
      (Default|OpenDoor _array_element)
      (bind _returnvalue (Rendering|Material|CreateDynamicMaterialInstance (Variables|Default|GetMEtaModel) 2 "/Game/Game/Materials/MI_dynamic_blueRed_neon.MI_dynamic_blueRed_neon" "None" :!class /Script/Engine.PrimitiveComponent))
      (bind _output_get (Variables|Default|SetdynamicColor _returnvalue))
      (Rendering|Material|SetVectorParameterValue _output_get "BaseColor" "(R=0.000000,G=1.000000,B=0.000000,A=1.000000)" :!class /Script/Engine.MaterialInstanceDynamic))))

(event OnComponentEndOverlap(trigger)
  (params (OverlappedComponent :type Primitive%20Component%20Object%20Reference) (OtherActor :type Actor%20Object%20Reference) (OtherComp :type Primitive%20Component%20Object%20Reference) (OtherBodyIndex :type Integer))
  ;[1 1 1] End Collision
  (Utilities|Casting|CastToBP_Perro OtherActor)
  (Variables|Default|SetplayerCollision false))

(event Custom|ActivateFinish
  ;[1 1 1] Init box color
  (bind _returnvalue (Rendering|Material|CreateDynamicMaterialInstance (Variables|Default|GetMEtaModel) 0 "/Game/Game/Materials/MI_dynamic_blueRed.MI_dynamic_blueRed" "None" :!class /Script/Engine.PrimitiveComponent))
  (bind _output_get (Variables|Default|SetdynamicColor _returnvalue))
  (Rendering|Material|SetVectorParameterValue _output_get "BaseColor" "(R=0.000000,G=1.000000,B=0.000000,A=1.000000)" :!class /Script/Engine.MaterialInstanceDynamic))

(fn ConstructionScript)