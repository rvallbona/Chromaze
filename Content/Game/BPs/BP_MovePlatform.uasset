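; BP_MovePlatform is a moving platform that shuttles endlessly between its saved start transform and EndPos.
; It starts on BeginPlay when Automatic is set, otherwise on the first Activate call, which also sets Automatic and plays a button sound at world origin.
; Two timelines chain each other on Finished, each lerping from the current transform toward its target, so motion compounds per update rather than following the curve directly.
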(event Custom|GoToStart
  ;[1 1 1] Go to Start
  (bind _newtrack_1 (Timeline|Timeline_0 PlayFromStart)
    (:Update
      (Transformation|SetActorTransform (Math|Transform|Lerp(Transform) (Transformation|GetActorTransform) (Variables|Default|GetStartPos) _newtrack_1)))
    (:Finished
      (CallFunction|GotoEnd))))

(event Custom|GoToEnd
  ;[1 1 1] Go To End
  (bind _newtrack_1 (Timeline|Timeline_1 PlayFromStart)
    (:Update
      (Transformation|SetActorTransform (Math|Transform|Lerp(Transform) (Transformation|GetActorTransform) (Variables|Default|GetEndPos) _newtrack_1)))
    (:Finished
      (CallFunction|GotoStart))))

(event Custom|Activate
  (if (not (Variables|Default|GetAutomatic))
    (CallFunction|GotoEnd)
    (Variables|Default|SetAutomatic true)
    (Audio|PlaySoundatLocation "/Game/Game/Sounds/FX/Button_Cue.Button_Cue" "0, 0, 0" "0, 0, 0" 1.0 1.0 0.0 0 0 0 0)))

(event EventBeginPlay
  ;[1 1 1] Save Start Position
  (Variables|Default|SetStartPos (Transformation|GetActorTransform))
  (if (Variables|Default|GetAutomatic)
    (CallFunction|GotoEnd)))

(fn ConstructionScript)