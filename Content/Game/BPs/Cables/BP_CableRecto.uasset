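; BP_CableRecto is a cable Blueprint whose neon mesh can be switched between black, blue and red.
; On BeginPlay it creates a dynamic instance of the blue/red neon material on the cable mesh and sets its BaseColor to black.
; The ChangeToBlue, ChangeToRed and ChangeToBlack events each create and store a fresh dynamic instance rather than reusing the existing one, then set its BaseColor.
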(event Custom|ChangeToBlue
  (bind _returnvalue (Rendering|Material|CreateDynamicMaterialInstance (Variables|Default|GetCableMesh) 0 "/Game/Game/Materials/MI_dynamic_blueRed_neon.MI_dynamic_blueRed_neon" "None" :!class /Script/Engine.PrimitiveComponent))
  (bind _output_get (Variables|Default|SetdynamicMaterialInstance _returnvalue))
  (Rendering|Material|SetVectorParameterValue _returnvalue "BaseColor" "(R=0.000000,G=0.000000,B=1.000000,A=1.000000)" :!class /Script/Engine.MaterialInstanceDynamic))

(event Custom|ChangeToRed
  (bind _returnvalue (Rendering|Material|CreateDynamicMaterialInstance (Variables|Default|GetCableMesh) 0 "/Game/Game/Materials/MI_dynamic_blueRed_neon.MI_dynamic_blueRed_neon" "None" :!class /Script/Engine.PrimitiveComponent))
  (bind _output_get (Variables|Default|SetdynamicMaterialInstance _returnvalue))
  (Rendering|Material|SetVectorParameterValue _returnvalue "BaseColor" "(R=1.000000,G=0.000000,B=0.000000,A=1.000000)" :!class /Script/Engine.MaterialInstanceDynamic))

(event Custom|ChangeToBlack
  (bind _returnvalue (Rendering|Material|CreateDynamicMaterialInstance (Variables|Default|GetCableMesh) 0 "/Game/Game/Materials/MI_dynamic_blueRed_neon.MI_dynamic_blueRed_neon" "None" :!class /Script/Engine.PrimitiveComponent))
  (bind _output_get (Variables|Default|SetdynamicMaterialInstance _returnvalue))
  (Rendering|Material|SetVectorParameterValue _returnvalue "BaseColor" "(R=0.000000,G=0.000000,B=0.000000,A=1.000000)" :!class /Script/Engine.MaterialInstanceDynamic))

(event EventBeginPlay
  (bind _returnvalue (Rendering|Material|CreateDynamicMaterialInstance (Variables|Default|GetCableMesh) 0 "/Game/Game/Materials/MI_dynamic_blueRed_neon.MI_dynamic_blueRed_neon" "None" :!class /Script/Engine.PrimitiveComponent))
  (bind _output_get (Variables|Default|SetdynamicMaterialInstance _returnvalue))
  (Rendering|Material|SetVectorParameterValue _returnvalue "BaseColor" "(R=0.000000,G=0.000000,B=0.000000,A=1.000000)" :!class /Script/Engine.MaterialInstanceDynamic))

(fn ConstructionScript)