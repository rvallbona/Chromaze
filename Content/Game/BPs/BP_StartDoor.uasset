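; BP_StartDoor is a start door Actor that opens by moving its Cube mesh along the Z axis.
; BeginPlay caches the Cube's initial relative transform.
; The OpenStartDoor event plays a 2D multimedia cue and a door-open sound at the world origin, then runs a timeline whose track adds a Z offset to the cached position.
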(event Custom|OpenStartDoor
  ;[1 1 1] Open Door
  (Audio|PlaySound2D "/Game/Game/Sounds/FX/Multimedia_Cue.Multimedia_Cue" 1.0 1.0 0.0 0 0)
  (Audio|PlaySoundatLocation "/Game/Game/Sounds/FX/Door-Open_Cue.Door-Open_Cue" "0, 0, 0" "0, 0, 0" 1.0 1.0 0.0 0 0 0 0)
  (bind _newtrack_2 (Timeline|Timeline_1 Play)
    (:Update
      (Transformation|SetRelativeLocation (Variables|Default|GetCube) (Math|Vector|MakeVector 0.0 0.0 (+ _newtrack_2 (.z (.location (Variables|Default|GetinitDoorTransform))))) false false))))

(event EventBeginPlay
  ;[1 1 1] Save Door Init Position
  (Variables|Default|SetinitDoorTransform (Transformation|GetRelativeTransform (Variables|Default|GetCube))))

(fn ConstructionScript)