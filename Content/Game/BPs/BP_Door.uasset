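; BP_Door is the level exit, opening on request and advancing the game once all players have entered its trigger.
; OpenDoor disables BP_Perro input, focuses BP_Camera, animates the Cube's height by timeline, then counts BP_Player actors and reactivates players through BP_GameManager.
; Box overlaps decrement that count and exits restore it.
; At zero, a second timeline moves the door to close and then calls NextLevel on the game manager.
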(event OnComponentBeginOverlap(Box)
  (params (OverlappedComponent :type Primitive%20Component%20Object%20Reference) (OtherActor :type Actor%20Object%20Reference) (OtherComp :type Primitive%20Component%20Object%20Reference) (OtherBodyIndex :type Integer) (bFromSweep :type Boolean) (SweepResult :type Hit%20Result%20Structure%20%28by%20ref%29))
  ;[1 1 1] Close Door And go next Level
  (Utilities|Casting|CastToBP_Player OtherActor)
  (bind _result (Math|Integer|DecrementInt (Variables|Default|GetplayerNum))
    (:%20%20
      (bind _output_get (Variables|Default|SetplayerNum _result))
      (if (<= _output_get 0)
        (Audio|PlaySoundatLocation "/Game/Game/Sounds/FX/Door-Open_Cue.Door-Open_Cue" "0, 0, 0" "0, 0, 0" 1.0 1.0 0.0 0 0 0 0)
        (bind _newtrack_2 (Timeline|Timeline_0 Play)
          (:Update
            (Transformation|SetRelativeLocation (Variables|Default|GetCube) (Math|Vector|MakeVector 0.0 0.0 (+ _newtrack_2 (.z (.location (Variables|Default|GetinitDoorTransform))))) false false))
          (:Finished
            ;[1 1 1] Go Next Level
            (bind _returnvalue (Actor|GetActorOfClass "/Game/Game/Levels/BP_GameManager.BP_GameManager_C"))
            (Utilities|IsValid _returnvalue
              (:Is%20Valid
                (Default|NextLevel _returnvalue)))))))))

(event OnComponentEndOverlap(Box)
  (params (OverlappedComponent :type Primitive%20Component%20Object%20Reference) (OtherActor :type Actor%20Object%20Reference) (OtherComp :type Primitive%20Component%20Object%20Reference) (OtherBodyIndex :type Integer))
  ;[1 1 1] End Overlap
  (Utilities|Casting|CastToBP_Player OtherActor)
  (bind _result (Math|Integer|IncrementInt (Variables|Default|GetplayerNum))
    (:%20%20
      (Variables|Default|SetplayerNum _result))))

(event Custom|OpenDoor
  ;[1 1 1] OpenDoor
  (if (not (Variables|Default|Getopen))
    (bind _returnvalue (Actor|GetActorOfClass "/Game/Game/Players/Blueprints/BP_Perro.BP_Perro_C"))
    (Input|DisableInput _returnvalue 0)
    (Variables|Default|Setopen true)
    (bind _returnvalue_2 (Actor|GetActorOfClass "/Game/Game/BPs/BP_Camera.BP_Camera_C"))
    (Default|FocusLastCamera _returnvalue_2)
    (Audio|PlaySoundatLocation "/Game/Game/Sounds/FX/Door-Open_Cue.Door-Open_Cue" (Transformation|GetActorLocation) "0, 0, 0" 1.0 1.0 0.0 0 0 0 0)
    (bind _newtrack_2 (Timeline|open_close Play)
      (:Update
        (Transformation|SetRelativeLocation (Variables|Default|GetCube) (Math|Vector|MakeVector 0.0 0.0 (+ _newtrack_2 (.z (.location (Variables|Default|GetinitDoorTransform))))) false false))
      (:Finished
        (bind _outactors (Actor|GetAllActorsOfClass "/Game/Game/Players/Blueprints/BP_Player.BP_Player_C"))
        (Variables|Default|SetplayerNum (Utilities|Array|Length _outactors))
        ;[1 1 1] ReActivate Players
        (bind _returnvalue_3 (Actor|GetActorOfClass "/Game/Game/Levels/BP_GameManager.BP_GameManager_C"))
        (Default|ActivatePlayers _returnvalue_3)))))

(event EventBeginPlay
  ;[1 1 1] Save Door Init Position
  (Variables|Default|SetinitDoorTransform (Transformation|GetRelativeTransform (Variables|Default|GetCube))))

(fn ConstructionScript)