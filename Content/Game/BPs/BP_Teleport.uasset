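; Teleporter actor that periodically moves everything inside its trigger to a linked destination, IdTp.
; A looping timeline started on BeginPlay animates the mesh color as a countdown, then calls Teleport and flashes a yellow neon material.
; Teleport captures overlapping actors, waits briefly, then moves each one, keeping its offset from the pad, rotation and scale.
; Each color change creates a new dynamic material instance, including on every timeline update.
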(event Custom|teleport
  (bind _returnvalue (Transformation|GetActorTransform))
  (bind _id_tp (Variables|Default|Getid_tp))
  (bind _returnvalue_2 (Transformation|GetActorTransform _id_tp))
  ;[1 1 1] Teleport
  (bind _output_get (Variables|Default|Settp_actorsObj (Collision|GetOverlappingActors (Variables|Default|Gettrigger) 0 :!class /Script/Engine.PrimitiveComponent)))
  (Utilities|FlowControl|Delay 0.1)
  (for _array_element _output_get
    (Transformation|SetActorTransform _array_element (Math|Transform|MakeTransform (Math|Vector|MakeVector (+ (.x (Math|Vector|MakeVector (- (.x (.location (Transformation|GetActorTransform _array_element))) (.x (.location _returnvalue))) (- (.y (.location (Transformation|GetActorTransform _array_element))) (.y (.location _returnvalue))) (- (.z (.location (Transformation|GetActorTransform _array_element))) (.z (.location _returnvalue))))) (.x (.location _returnvalue_2))) (+ (.y (Math|Vector|MakeVector (- (.x (.location (Transformation|GetActorTransform _array_element))) (.x (.location _returnvalue))) (- (.y (.location (Transformation|GetActorTransform _array_element))) (.y (.location _returnvalue))) (- (.z (.location (Transformation|GetActorTransform _array_element))) (.z (.location _returnvalue))))) (.y (.location _returnvalue_2))) (+ (.z (Math|Vector|MakeVector (- (.x (.location (Transformation|GetActorTransform _array_element))) (.x (.location _returnvalue))) (- (.y (.location (Transformation|GetActorTransform _array_element))) (.y (.location _returnvalue))) (- (.z (.location (Transformation|GetActorTransform _array_element))) (.z (.location _returnvalue))))) (.z (.location _returnvalue_2)))) (.rotation (Transformation|GetActorTransform _array_element)) (.scale (Transformation|GetActorTransform _array_element))) false true)))

(event EventBeginPlay
  (bind _newtrack_0 (Timeline|delaaay PlayFromStart)
    (:Update
      (bind _returnvalue (Rendering|Material|CreateDynamicMaterialInstance (Variables|Default|Getmesh) 0 "/Game/Game/Materials/MI_dynamic_blueRed.MI_dynamic_blueRed" "None" :!class /Script/Engine.PrimitiveComponent))
      (Rendering|Material|SetVectorParameterValue _returnvalue "BaseColor" (Utilities|Struct|MakeLinearColor 1.0 _newtrack_0 0.0 1.0) :!class /Script/Engine.MaterialInstanceDynamic))
    (:Finished
      (CallFunction|Teleport)
      (bind _returnvalue_2 (Rendering|Material|CreateDynamicMaterialInstance (Variables|Default|Getmesh) 0 "/Game/Game/Materials/MI_dynamic_blueRed_neon.MI_dynamic_blueRed_neon" "None" :!class /Script/Engine.PrimitiveComponent))
      (Rendering|Material|SetVectorParameterValue _returnvalue_2 "BaseColor" "(R=1.000000,G=1.000000,B=0.000000,A=1.000000)" :!class /Script/Engine.MaterialInstanceDynamic)
      (Timeline|delaaay PlayFromStart))))

(fn ConstructionScript)