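; Game mode for a two-player game that spawns and possesses BP_Player pawns on a shared game camera.
; On BeginPlay it caches two spawn transforms from the first entries of BP_GameManager's level spawn arrays.
; SpawnPlayer replaces a controller's existing pawn, alternating spawns via FlipFlop and setting color and controller ID.
; Once the player count reaches the maximum, it has the manager destroy the spawn message.
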(event Custom|SpawnPlayer
  (params (PlayerController :type Player%20Controller%20Object%20Reference))
  (bind _returnvalue (Class|GameplayStatics|GetPlayerControllerID PlayerController))
  (bind _returnvalue_2 (Pawn|GetControlledPawn PlayerController))
  ;[1 1 1] SpawnPlayer
  (if (< (Variables|Default|GetCurrentPlayers) (Variables|Default|GetMaxPlayers))
    (Utilities|IsValid _returnvalue_2
      (:Is%20Valid
        (Actor|DestroyActor _returnvalue_2)
        (Utilities|FlowControl|FlipFlop
          (:A
            (bind _returnvalue_3 (Game|SpawnActorfromClass "/Game/Game/Players/Blueprints/BP_Player.BP_Player_C" (Variables|Default|Getspawn0) "Undefined" 0 0))
            (Pawn|Possess PlayerController _returnvalue_3)
            (Default|SetColor _returnvalue_3 (== (Variables|Default|GetCurrentPlayers) 0))
            (Variables|/Game/Game/Players/Blueprints/BP_Player.BP_Player_C|Setid _returnvalue_3 _returnvalue))
          (:B
            (bind _returnvalue_4 (Game|SpawnActorfromClass "/Game/Game/Players/Blueprints/BP_Player.BP_Player_C" (Variables|Default|Getspawn1) "Undefined" 0 0))
            (Pawn|Possess PlayerController _returnvalue_4)
            (Default|SetColor _returnvalue_4 (== (Variables|Default|GetCurrentPlayers) 0))
            (Variables|/Game/Game/Players/Blueprints/BP_Player.BP_Player_C|Setid _returnvalue_4 _returnvalue)))
        (Game|Player|SetViewTargetwithBlend PlayerController (Variables|Default|GetGameCamera) 0.0 "VTBlend_Linear" 0.0 false)
        (bind _result (Math|Integer|IncrementInt (Variables|Default|GetCurrentPlayers))
          (:%20%20
            (bind _output_get (Variables|Default|SetCurrentPlayers _result))
            (if (>= _output_get (Variables|Default|GetMaxPlayers))
              (bind _returnvalue_5 (Actor|GetActorOfClass "/Game/Game/Levels/BP_GameManager.BP_GameManager_C"))
              (Default|DestroySpawnMessage _returnvalue_5))))))))

(event EventBeginPlay
  ;[1 1 1] Set spawnPoints
  (bind _returnvalue (Actor|GetActorOfClass "/Game/Game/Levels/BP_GameManager.BP_GameManager_C"))
  (Variables|Default|Setspawn0 (Utilities|Array|Get(acopy) (Variables|/Game/Game/Levels/BP_GameManager.BP_GameManager_C|GetlevelsSpawns _returnvalue)))
  (Variables|Default|Setspawn1 (Utilities|Array|Get(acopy) (Variables|/Game/Game/Levels/BP_GameManager.BP_GameManager_C|GetlevelsSpawns_1 _returnvalue))))

(fn ConstructionScript)