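; Level manager for a two-player game that runs the level order and handles switching between players and a shared dog.
; NextLevel teleports both players, sets cameras, opens the matching start door and destroys the dog, or shows the win screen and returns to the main menu.
; When both level finishes are occupied, player 0 possesses a spawned or existing dog, player 1 gets its jump, and dog finishes activate.
; ActivatePlayers restores player control.
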(event Custom|NextLevel
  (bind _returnvalue (Game|GetPlayerController 0))
  (bind _levelsspawns (Variables|Default|GetlevelsSpawns))
  (bind _levelsspawns_1 (Variables|Default|GetlevelsSpawns_1))
  (bind _currentlevel (Variables|Default|GetCurrentLevel))
  (bind _levelorder (Variables|Default|GetlevelOrder))
  (bind _currentlevel_2 (Variables|Default|GetCurrentLevel))
  (bind _levelorder_2 (Variables|Default|GetlevelOrder))
  (bind _currentlevel_3 (Variables|Default|GetCurrentLevel))
  (bind _output (Utilities|Array|Get(acopy) _levelorder _currentlevel))
  (bind _output_2 (Utilities|Array|Get(acopy) _levelorder_2 _currentlevel_2))
  (bind _output_3 (Utilities|Array|Get(acopy) _levelsspawns_1 _output_2))
  (bind _output_4 (Utilities|Array|Get(acopy) _levelsspawns _output))
  ;[1 1 1] Next Level
  (Math|Integer|IncrementInt _currentlevel_3
    (:%20%20
      (if (< _currentlevel_3 (Utilities|Array|Length (Variables|Default|GetlevelOrder)))
        (bind _outactors (Actor|GetAllActorsOfClass "/Game/Game/Players/Blueprints/BP_Player.BP_Player_C"))
        (for (_array_element _array_index) _outactors
          (if (== _array_index 0)
            (Transformation|SetActorTransform _array_element _output_4 false true)
            (Variables|/Game/Game/Players/Blueprints/BP_Player.BP_Player_C|SetinitTransform _array_element _output_4)
            (else
              (Transformation|SetActorTransform _array_element _output_3 false true)
              (Variables|/Game/Game/Players/Blueprints/BP_Player.BP_Player_C|SetinitTransform _array_element _output_3))))
        ;[1 1 1] Init cameras
        (bind _returnvalue_2 (Actor|GetActorOfClass "/Game/Game/BPs/BP_Camera.BP_Camera_C"))
        (Default|SetLevelCameras _returnvalue_2 (Utilities|Array|Get(acopy) (Variables|Default|GetlevelOrder) (Variables|Default|GetCurrentLevel)))
        (Utilities|FlowControl|Delay 0.5)
        ;[1 1 1] Open start level Door
        (bind _outactors_2 (Actor|GetAllActorsOfClass "/Game/Game/BPs/BP_StartDoor.BP_StartDoor_C"))
        (for _array_element_2 _outactors_2
          (bind _asbp_start_door (Utilities|Casting|CastToBP_StartDoor _array_element_2))
          (if (== (Variables|/Game/Game/BPs/BP_StartDoor.BP_StartDoor_C|Getlevel _asbp_start_door) (Utilities|Array|Get(acopy) (Variables|Default|GetlevelOrder) (Variables|Default|GetCurrentLevel)))
            (Default|OpenStartDoor _asbp_start_door)
            ;[1 1 1] Destruir al perro
            (bind _returnvalue_3 (Actor|GetActorOfClass "/Game/Game/Players/Blueprints/BP_Perro.BP_Perro_C"))
            (Utilities|IsValid _returnvalue_3
              (:Is%20Valid
                (Actor|DestroyActor _returnvalue_3)))))
        (else
          (bind _returnvalue_4 (UserInterface|CreateWidget "/Game/Game/UI/WIn.WIn_C"))
          (UserInterface|Viewport|AddtoViewport _returnvalue_4 0)
          (Utilities|FlowControl|Delay 3.0)
          (Game|OpenLevel(byName) "MainMenuMap")
          (Variables|/Script/Engine.PlayerController|SetbShowMouseCursor _returnvalue false)
          (Input|SetInputModeGameOnly _returnvalue))))))

(event Custom|DestroySpawnMessage
  (Widget|RemovefromParent (stale EventBeginPlay _returnvalue)))

(event Custom|ActivateDog
  ;[1 1 1] Activate Dog
  (Variables|Default|SetactiveFinishes 2)
  (bind _outactors (Actor|GetAllActorsOfClass "/Game/Game/BPs/BP_Finish.BP_Finish_C"))
  (for _array_element _outactors
    (if (== (Variables|/Game/Game/BPs/BP_Finish.BP_Finish_C|Getlevel _array_element) (Utilities|Array|Get(acopy) (Variables|Default|GetlevelOrder) (Variables|Default|GetCurrentLevel)))
      (if (Variables|/Game/Game/BPs/BP_Finish.BP_Finish_C|GetplayerCollision _array_element)
        (bind _result (Math|Integer|DecrementInt (Variables|Default|GetactiveFinishes))
          (:%20%20
            (Variables|Default|SetactiveFinishes _result))))))
  (if (<= (Variables|Default|GetactiveFinishes) 0)
    (Utilities|IsValid (Variables|Default|GetdogObject)
      (:Is%20Valid
        (CallFunction|ControllExistingDog))
      (:Is%20Not%20Valid
        (CallFunction|SpawnNewDog)))
    (bind _outactors_2 (Actor|GetAllActorsOfClass "/Game/Game/BPs/BP_Dog_Finish.BP_Dog_Finish_C"))
    (for _array_element_2 _outactors_2
      (if (== (Variables|/Game/Game/BPs/BP_Dog_Finish.BP_Dog_Finish_C|Getlevel _array_element_2) (Utilities|Array|Get(acopy) (Variables|Default|GetlevelOrder) (Variables|Default|GetCurrentLevel)))
        (Default|ActivateFinish _array_element_2)))))

(event Custom|ActivatePlayers
  (bind _returnvalue (Game|GetPlayerController 0))
  ;[1 1 1] ActivatePlayers
  (Audio|PlaySound2D "/Game/Game/Sounds/FX/beep2_Cue.beep2_Cue" 1.0 1.0 0.0 0 0)
  (bind _outactors (Actor|GetAllActorsOfClass "/Game/Game/Players/Blueprints/BP_Player.BP_Player_C"))
  (for _array_element _outactors
    (if (== (Variables|/Game/Game/Players/Blueprints/BP_Player.BP_Player_C|Getid _array_element) 0)
      (Pawn|Possess _returnvalue _array_element)
      (Input|EnableInput _array_element 0)
      (bind _asbp_2players_game_mode (Utilities|Casting|CastToBP_2Players_GameMode (Game|GetGameMode)))
      (Game|Player|SetViewTargetwithBlend _returnvalue (Variables|/Game/Game/Players/Blueprints/BP_2Players_GameMode.BP_2Players_GameMode_C|GetGameCamera _asbp_2players_game_mode) 0.0 "VTBlend_Linear" 0.0 false)
      (else
        (Variables|/Game/Game/Players/Blueprints/BP_Player.BP_Player_C|SetcontrollingDogJump _array_element false)))))

(event EventBeginPlay
  ;[1 1 1] Tutorial Message
  (bind _returnvalue (UserInterface|CreateWidget "/Game/Game/UI/SpawnMessage.SpawnMessage_C"))
  (UserInterface|Viewport|AddtoViewport _returnvalue 0))

(fn ConstructionScript)

(fn ControllExistingDog
  (bind _returnvalue (Game|GetPlayerController 0))
  (Audio|PlaySound2D "/Game/Game/Sounds/FX/beep_Cue.beep_Cue" 1.0 1.0 0.0 0 0)
  (bind _outactors (Actor|GetAllActorsOfClass "/Game/Game/Players/Blueprints/BP_Player.BP_Player_C"))
  (for _array_element _outactors
    (if (== (Variables|/Game/Game/Players/Blueprints/BP_Player.BP_Player_C|Getid _array_element) 0)
      (Input|DisableInput _array_element 0)
      (Pawn|Possess _returnvalue (Variables|Default|GetdogObject))
      (bind _returnvalue_2 (Actor|GetActorOfClass "/Game/Game/BPs/BP_Camera.BP_Camera_C"))
      (Game|Player|SetViewTargetwithBlend _returnvalue _returnvalue_2 0.0 "VTBlend_Linear" 0.0 false)
      (bind _outactors_2 (Actor|GetAllActorsOfClass "/Game/Game/Players/Blueprints/BP_Player.BP_Player_C"))
      (for _array_element_2 _outactors_2
        (if (== (Variables|/Game/Game/Players/Blueprints/BP_Player.BP_Player_C|Getid _array_element_2) 1)
          (Variables|/Game/Game/Players/Blueprints/BP_Player.BP_Player_C|SetcontrollingDogJump _array_element_2 true))))))

(fn SpawnNewDog
  (bind _returnvalue (Game|GetPlayerController 0))
  (Audio|PlaySound2D "/Game/Game/Sounds/FX/beep_Cue.beep_Cue" 1.0 1.0 0.0 0 0)
  (bind _outactors (Actor|GetAllActorsOfClass "/Game/Game/Players/Blueprints/BP_Player.BP_Player_C"))
  (for _array_element _outactors
    (if (== (Variables|/Game/Game/Players/Blueprints/BP_Player.BP_Player_C|Getid _array_element) 0)
      (Input|DisableInput _array_element 0)
      (bind _returnvalue_2 (Game|SpawnActorfromClass "/Game/Game/Players/Blueprints/BP_Perro.BP_Perro_C" (Utilities|Array|Get(acopy) (Variables|Default|GetlevelsSpawns_perro) (Utilities|Array|Get(acopy) (Variables|Default|GetlevelOrder) (Variables|Default|GetCurrentLevel))) "Undefined" 0 0))
      (bind _output_get (Variables|Default|SetdogObject _returnvalue_2))
      (Pawn|Possess _returnvalue _output_get)
      (bind _returnvalue_3 (Actor|GetActorOfClass "/Game/Game/BPs/BP_Camera.BP_Camera_C"))
      (Game|Player|SetViewTargetwithBlend _returnvalue _returnvalue_3 0.0 "VTBlend_Linear" 0.0 false)
      (bind _outactors_2 (Actor|GetAllActorsOfClass "/Game/Game/Players/Blueprints/BP_Player.BP_Player_C"))
      (for _array_element_2 _outactors_2
        (if (== (Variables|/Game/Game/Players/Blueprints/BP_Player.BP_Player_C|Getid _array_element_2) 1)
          (Variables|/Game/Game/Players/Blueprints/BP_Player.BP_Player_C|SetcontrollingDogJump _array_element_2 true))))))